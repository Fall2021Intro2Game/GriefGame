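; Player controller that handles the player's death by bringing up the game-over screen.
; OnDeath unpossesses the pawn and starts the death montage partway in.
; Both the montage node's immediate output and its Notify End create the game-over widget, show the cursor, pause the game and destroy the controller, so the screen does not wait for the animation.
; Delayed widget-removal and game-restart chains are left unconnected.
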(event Custom|OnDeath
  (Pawn|UnPossess)
  (Animation|Montage|PlayMontage 0 "/Game/Voodoo_Doll/Animations/Death_Montage.Death_Montage" 1.0 1.0
    (:then
      _)
    (:OnNotifyEnd
      _))
  (bind _returnvalue (UserInterface|CreateWidget "/Game/GameoverScreen/Gameover_Sceen_Widget.Gameover_Sceen_Widget_C" self))
  (UserInterface|Viewport|AddtoViewport _returnvalue 0)
  (Variables|Default|SetbShowMouseCursor true)
  (Game|SetGamePaused true)
  (Actor|DestroyActor))

(event EventBeginPlay)

(event EventTick
  (params (DeltaSeconds :type Float%20%28single-precision%29)))

(fn ConstructionScript)