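; Enemy AI character that chases the SideScrollerCharacter and plays an attack montage when it comes within range.
; After BeginPlay it caches the first SideScrollerCharacter found following a short delay, while a looping AI MoveTo polls until that target is valid, then keeps pursuing it.
; AttackRange overlaps toggle CanAttack, and the montage replays on completion while the target stays inside; no damage is applied here.
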(event OnComponentBeginOverlap(AttackRange)
  (params (OverlappedComponent :type Primitive%20Component%20Object%20Reference) (OtherActor :type Actor%20Object%20Reference) (OtherComp :type Primitive%20Component%20Object%20Reference) (OtherBodyIndex :type Integer) (bFromSweep :type Boolean) (SweepResult :type Hit%20Result%20Structure%20%28by%20ref%29))
  (if (and (== OtherActor (Variables|Default|GetMyEnemy)) (not (Variables|Default|GetIsAttacking)))
    (Variables|Default|SetCanAttack true)
    (Variables|Default|SetIsAttacking true :!label _label)
    (Animation|Montage|PlayMontage (Variables|Character|GetMesh) "/Game/Characters/AI/Animation/scp_attack_Montage.scp_attack_Montage"
      (:OnCompleted
        (Variables|Default|SetIsAttacking false)
        (if (Variables|Default|GetCanAttack)
          (goto _label))))))

(event OnComponentEndOverlap(AttackRange)
  (params (OverlappedComponent :type Primitive%20Component%20Object%20Reference) (OtherActor :type Actor%20Object%20Reference) (OtherComp :type Primitive%20Component%20Object%20Reference) (OtherBodyIndex :type Integer))
  (if (and (== OtherActor (Variables|Default|GetMyEnemy)) (Variables|Default|GetCanAttack))
    (Variables|Default|SetCanAttack false)))

(event Custom|Get_Enemy
  (Utilities|FlowControl|Delay 1.0)
  (bind _outactors (Actor|GetAllActorsOfClass "/Game/SideScrollerBP/Blueprints/SideScrollerCharacter.SideScrollerCharacter_C"))
  (Variables|Default|SetMyEnemy (Utilities|Array|Get(acopy) _outactors)))

(event Custom|BaseMovement
  (Utilities|IsValid (Variables|Default|GetMyEnemy) :!label _label
    (:Is%20Valid
      (AI|AIMoveTo self "0, 0, 0" (Variables|Default|GetMyEnemy) 3e+01 false
        (:OnSuccess
          (Utilities|FlowControl|Delay 2.0)
          (goto _label))
        (:OnFail
          (goto _label))))
    (:Is%20Not%20Valid
      (Utilities|FlowControl|Delay 1.0)
      (goto _label))))

(event EventBeginPlay
  (Utilities|FlowControl|Sequence
    (:then_0
      (CallFunction|GetEnemy))
    (:then_1
      (CallFunction|BaseMovement))))

(fn ConstructionScript)